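; BP_Player is the player Blueprint, handling gun attachment and an aim camera.
; On BeginPlay it attaches the gun component to a socket on the mesh.
; Aim start plays a timeline that drives the spring arm length, and aim end reverses it for a smooth camera transition.
; Tick prints the aiming state to the screen as debug output.
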(event EventBeginPlay
  (Transformation|AttachComponentToComponent (Variables|Default|GetGunComponent) (Variables|Character|GetMesh) (Variables|Default|GetAttachSocket) "SnapToTarget" "KeepRelative" "KeepRelative" true))

(event EventTick
  (params (DeltaSeconds :type Float%20%28single-precision%29))
  (Development|PrintString (Utilities|String|ToString(Boolean) (Class|PlayerCharacter|IsAiming)) true true "(R=0.000000,G=0.660000,B=1.000000,A=1.000000)" 0.1))

(event EventOnAimStarted
  (bind _camera_arm_length (Timeline|Camera%20Timeline Play)
    (:Update
      (Variables|/Script/Engine.SpringArmComponent|SetTargetArmLength (Variables|Default|GetSpringArmComponent) _camera_arm_length))))

(event EventOnAimEnded
  (bind _camera_arm_length (Timeline|Camera%20Timeline Reverse)
    (:Update
      (Variables|/Script/Engine.SpringArmComponent|SetTargetArmLength (Variables|Default|GetSpringArmComponent) _camera_arm_length))))

(fn ConstructionScript)